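; Anim notify that plays a footstep haptic on the player's controller when an animation reaches it.
; It casts player pawn 0 to BP_Character and fires the ForceFeedbackEffect variable, non-looping, only while movement speed is below 600.
; It ignores the notifying mesh, so the check and the rumble always target player 0, whichever mesh triggers it.
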(fn ReceivedNotify
  (params (MeshComp :type Skeletal%20Mesh%20Component%20Object%20Reference) (Animation :type Anim%20Sequence%20Base%20Object%20Reference) (EventReference :type Anim%20Notify%20Event%20Reference%20Structure%20%28by%20ref%29))
  (if (not (>= (Math|Vector|VectorLength (Variables|/Script/Engine.MovementComponent|GetVelocity (Variables|/Script/Engine.Character|GetCharacterMovement (.AsBP%20Character (Utilities|Casting|CastToBP_Character (Game|Player|GetPlayerPawn 0)))))) 6e+02))
    (Game|Feedback|ClientPlayForceFeedback (Game|GetPlayerController 0) (Variables|Default|GetForce%20Feedback%20Effect) "None" false false false)
    (return false)))