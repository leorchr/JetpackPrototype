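; Player controller that switches Enhanced Input mappings as the player enters and exits the spaceship.
; On BeginPlay it adds the main mapping context, finds the BP_SpaceShipPawn in the level and binds to its enter and exit events.
; Those events swap between the spaceship and hovering mapping contexts and update the PawnPossessed enum to track the current mode.
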(event Custom|NormalMode
  (bind _returnvalue (PlayerController|LocalPlayerSubsystems|GetEnhancedInputLocalPlayerSubsystem))
  (Input|RemoveMappingContext _returnvalue "/Game/GameManager/Inputs/IMC_SpaceShip.IMC_SpaceShip" "(bIgnoreAllPressedKeysUntilRelease=True,bForceImmediately=False,bNotifyUserSettings=False)")
  (Input|AddMappingContext _returnvalue "/Game/FirstPerson/Input/IMC_Hovering.IMC_Hovering" 0 "(bIgnoreAllPressedKeysUntilRelease=True,bForceImmediately=False,bNotifyUserSettings=False)")
  (Variables|Default|SetPawnPossessed "NewEnumerator0"))

(event Custom|SpaceShipMode
  (bind _returnvalue (PlayerController|LocalPlayerSubsystems|GetEnhancedInputLocalPlayerSubsystem))
  (Input|RemoveMappingContext _returnvalue "/Game/FirstPerson/Input/IMC_Hovering.IMC_Hovering" "(bIgnoreAllPressedKeysUntilRelease=True,bForceImmediately=False,bNotifyUserSettings=False)")
  (Input|AddMappingContext _returnvalue "/Game/GameManager/Inputs/IMC_SpaceShip.IMC_SpaceShip" 0 "(bIgnoreAllPressedKeysUntilRelease=True,bForceImmediately=False,bNotifyUserSettings=False)")
  (Variables|Default|SetPawnPossessed "NewEnumerator1"))

(event EventBeginPlay
  (Input|AddMappingContext (PlayerController|LocalPlayerSubsystems|GetEnhancedInputLocalPlayerSubsystem) "/Game/GameManager/Inputs/IMC_Main.IMC_Main" 0 "(bIgnoreAllPressedKeysUntilRelease=True,bForceImmediately=False,bNotifyUserSettings=False)")
  (bind _returnvalue (Actor|GetActorOfClass "/Game/Blueprints/SpaceShip/BP_SpaceShipPawn.BP_SpaceShipPawn_C"))
  (Utilities|IsValid _returnvalue
    (:Is%20Valid
      (EventDispatchers|BindEventtoEnterSpaceShip _returnvalue (delegate Custom|SpaceShipMode))
      (EventDispatchers|BindEventtoExitSpaceShip _returnvalue (delegate Custom|NormalMode)))))

(fn ConstructionScript)