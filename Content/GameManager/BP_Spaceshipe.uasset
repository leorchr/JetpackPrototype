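; BP_Spaceshipe is a spaceship pawn that the player can approach and take control of.
; While it is not player-controlled, its ControlTrigger overlaps show or hide a lazily created prompt widget and register or clear it as the player's interactable through messages.
; StartInteraction possesses the ship with the first player controller, hides the prompt, then disables the driver's collision and attaches them to the trigger.
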(event OnComponentBeginOverlap(ControlTrigger)
  (params (OverlappedComponent :type Primitive%20Component%20Object%20Reference) (OtherActor :type Actor%20Object%20Reference) (OtherComp :type Primitive%20Component%20Object%20Reference) (OtherBodyIndex :type Integer) (bFromSweep :type Boolean) (SweepResult :type Hit%20Result%20Structure%20%28by%20ref%29))
  (if (not (Pawn|IsPlayerControlled self))
    (bind _yes (Class|BPICharacter|IsPlayer(Message) OtherActor))
    (if _yes
      (CallFunction|ToggleInstructionWidget true)
      (Class|BPICharacter|SetInteractable(Message) OtherActor self))))

(event OnComponentEndOverlap(ControlTrigger)
  (params (OverlappedComponent :type Primitive%20Component%20Object%20Reference) (OtherActor :type Actor%20Object%20Reference) (OtherComp :type Primitive%20Component%20Object%20Reference) (OtherBodyIndex :type Integer))
  (if (not (Pawn|IsPlayerControlled self))
    (bind _yes (Class|BPICharacter|IsPlayer(Message) OtherActor))
    (if _yes
      (CallFunction|ToggleInstructionWidget false)
      (Class|BPICharacter|SetInteractable(Message) OtherActor))))

(event EventStartInteraction
  (params (InteractingCharacter :type Character%20Object%20Reference))
  (Variables|Default|SetDriver InteractingCharacter)
  (Pawn|Possess (Game|GetPlayerController 0) self)
  (CallFunction|ToggleInstructionWidget false)
  (Collision|SetActorEnableCollision (Variables|Default|GetDriver) false)
  (Transformation|AttachComponentToComponent (Variables|Default|GetDriver) (Variables|Default|GetControlTrigger) "None" "KeepWorld" "KeepWorld" "KeepWorld" true))

(fn ConstructionScript)

(fn ToggleInstructionWidget
  (params (Show%20/Hide :type Boolean))
  (if Show%20/Hide
    (Variables|Default|GetWdgInstruction
      (:then
        _)
      (:else
        (bind _returnvalue (UserInterface|CreateWidget "/Game/Character/Interfaces/W_SpaceshipInteract.W_SpaceshipInteract_C" (Game|GetPlayerController 0)))
        (Variables|Default|SetWdgInstruction _returnvalue)))
    (UserInterface|Viewport|AddtoViewport (Variables|Default|GetWdgInstruction) 0)
    (else
      (bind _wdginstruction (Variables|Default|GetWdgInstruction)
        (:then
          (if (UserInterface|Viewport|IsinViewport _wdginstruction)
            (Widget|RemovefromParent _wdginstruction)))
        (:else)))))