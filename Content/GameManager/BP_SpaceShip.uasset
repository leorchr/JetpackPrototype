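; BP_SpaceShip is a spaceship that the player can board, control through possession and exit.
; Overlapping its ControlTrigger while unoccupied shows an interact prompt widget and registers the ship as the player's interactable through messages.
; StartInteraction possesses the ship, then attaches and hides the driver with collision and mesh shadow off.
; IA_Interact re-possesses the driver and restores visibility, collision and shadow, without an explicit detach.
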(event OnComponentBeginOverlap(ControlTrigger)
  (params (OverlappedComponent :type Primitive%20Component%20Object%20Reference) (OtherActor :type Actor%20Object%20Reference) (OtherComp :type Primitive%20Component%20Object%20Reference) (OtherBodyIndex :type Integer) (bFromSweep :type Boolean) (SweepResult :type Hit%20Result%20Structure%20%28by%20ref%29))
  ;[0 1 0.1794] Player enter collision
  (if (not (Pawn|IsPlayerControlled self))
    (bind _yes (Class|BPICharacter|IsPlayer(Message) OtherActor))
    (if _yes
      (CallFunction|ToggleInstructionWidget true)
      (Class|BPICharacter|SetInteractable(Message) OtherActor self))))

(event OnComponentEndOverlap(ControlTrigger)
  (params (OverlappedComponent :type Primitive%20Component%20Object%20Reference) (OtherActor :type Actor%20Object%20Reference) (OtherComp :type Primitive%20Component%20Object%20Reference) (OtherBodyIndex :type Integer))
  ;[1 0 0] Player exit collision
  (if (not (Pawn|IsPlayerControlled self))
    (bind _yes (Class|BPICharacter|IsPlayer(Message) OtherActor))
    (if _yes
      (CallFunction|ToggleInstructionWidget false)
      (Class|BPICharacter|SetInteractable(Message) OtherActor))))

(event Input|EnhancedActionEvents|EnhancedInputActionIA_Interact
  (params (ActionValue :type Boolean) (ElapsedSeconds :type Float%20%28double-precision%29) (TriggeredSeconds :type Float%20%28double-precision%29) (InputAction :type Input%20Action%20Object%20Reference :default "/Game/GameManager/Inputs/IA_Interact.IA_Interact"))
  ;[0.5167 1 0.701] Interact input
  (:Started
    (bind _driver (Variables|Default|GetDriver)
      (:then
        (Collision|SetActorEnableCollision _driver true)
        (Pawn|Possess (Game|GetPlayerController 0) _driver)
        ;;[0 1 0.026] Enable Mesh, Collision, Shadow
        (Rendering|SetActorHiddenInGame _driver false)
        (Collision|SetCollisionEnabled (Variables|/Script/Engine.Character|GetCapsuleComponent _driver) "QueryAndPhysics")
        (Rendering|SetCastShadow (Variables|/Script/Engine.Character|GetMesh _driver) true)
        (Variables|Default|SetInSpaceShip false))
      (:else))))

(event EventStartInteraction
  (params (InteractingCharacter :type Character%20Object%20Reference))
  ;[0.1498 0.9003 1] Start Interaction
  (Variables|Default|SetDriver InteractingCharacter)
  (Pawn|Possess (Game|GetPlayerController 0) self)
  (CallFunction|ToggleInstructionWidget false)
  (Collision|SetActorEnableCollision (Variables|Default|GetDriver) false)
  (Transformation|AttachComponentToComponent (Variables|Default|GetDriver) (Variables|Default|GetControlTrigger) "None" "KeepWorld" "KeepWorld" "KeepWorld" true)
  ;;[1 0 0] Disable Mesh, Collision, Shadow
  (Rendering|SetActorHiddenInGame (Variables|Default|GetDriver) true)
  (Collision|SetCollisionEnabled (Variables|/Script/Engine.Character|GetCapsuleComponent (Variables|Default|GetDriver)) "NoCollision")
  (Rendering|SetCastShadow (Variables|/Script/Engine.Character|GetMesh (Variables|Default|GetDriver)) false)
  (Variables|Default|SetInSpaceShip true))

(fn ConstructionScript)

(fn ToggleInstructionWidget
  (params (Show%20/Hide :type Boolean))
  (if Show%20/Hide
    (Variables|Default|GetWdgInstruction
      (:then
        _)
      (:else
        (bind _returnvalue (UserInterface|CreateWidget "/Game/Character/Interfaces/W_SpaceshipInteract.W_SpaceshipInteract_C" (Game|GetPlayerController 0)))
        (Variables|Default|SetWdgInstruction _returnvalue)))
    (UserInterface|Viewport|AddtoViewport (Variables|Default|GetWdgInstruction) 0)
    (else
      (bind _wdginstruction (Variables|Default|GetWdgInstruction)
        (:then
          (if (UserInterface|Viewport|IsinViewport _wdginstruction)
            (Widget|RemovefromParent _wdginstruction)))
        (:else)))))