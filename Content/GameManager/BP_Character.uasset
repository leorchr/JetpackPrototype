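; Player character Blueprint with jetpack-aware movement, sensitivity-scaled look with clamped pitch, and interaction.
; AC_Jetpack turbo power rescales move input to limit steering and hides the mesh below a threshold.
; Jetpack events drive landing shake and spawn rocket exhaust Niagara systems on hover start; walking start also shakes the camera.
; Interact calls the registered PossibleInteract and adds the hovering input context; the turbo-stop handler currently has no effect.
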(event Input|EnhancedActionEvents|EnhancedInputActionIA_Move
  (params (ActionValue :type Vector%202D%20Structure) (ElapsedSeconds :type Float%20%28double-precision%29) (TriggeredSeconds :type Float%20%28double-precision%29) (InputAction :type Input%20Action%20Object%20Reference :default "/Game/GameManager/Inputs/IA_Move.IA_Move"))
  (bind _returnvalue (Transformation|GetActorRotation))
  (bind _ac_jetpack (Variables|Default|GetAC_Jetpack))
  (bind _turbo_pwr (Default|JPTurboPwr _ac_jetpack))
  ;[0 0.5128 1] MOVEMENT
  (Pawn|Input|AddMovementInput (Math|Vector|GetForwardVector (Math|Rotator|MakeRotator 0.0 0.0 (.yaw (Transformation|GetActorRotation)))) (Math|Float|MapRangeClamped _turbo_pwr 0.0 1.0 (.y ActionValue) 0.0) false)
  (Pawn|Input|AddMovementInput (Math|Vector|GetRightVector (Math|Rotator|MakeRotator (.roll _returnvalue) 0.0 (.yaw _returnvalue))) (Math|Float|MapRangeClamped _turbo_pwr 0.0 1.0 (.x ActionValue) 0.0) false))

(event Input|EnhancedActionEvents|EnhancedInputActionIA_Look
  (params (ActionValue :type Vector%202D%20Structure) (ElapsedSeconds :type Float%20%28double-precision%29) (TriggeredSeconds :type Float%20%28double-precision%29) (InputAction :type Input%20Action%20Object%20Reference :default "/Game/GameManager/Inputs/IA_Look.IA_Look"))
  ;[0 1 0.03071] CAMERA
  (Pawn|Input|AddControllerPitchInput (* (.y ActionValue) (Variables|Default|GetVertical%20Sensitivity%20Multiplier)))
  (Pawn|Input|AddControllerYawInput (* (.x ActionValue) (Variables|Default|GetHorizontal%20Sensitivity%20Multiplier))))

(event Input|EnhancedActionEvents|EnhancedInputActionIA_Interact
  (params (ActionValue :type Boolean) (ElapsedSeconds :type Float%20%28double-precision%29) (TriggeredSeconds :type Float%20%28double-precision%29) (InputAction :type Input%20Action%20Object%20Reference :default "/Game/GameManager/Inputs/IA_Interact.IA_Interact"))
  (bind _possibleinteract (Variables|Default|GetPossibleInteract))
  ;[0.5792 0.2181 1] INTERACT
  (:Started
    (Utilities|IsValid _possibleinteract
      (:Is%20Valid
        (Input|AddMappingContext (PlayerController|LocalPlayerSubsystems|GetEnhancedInputLocalPlayerSubsystem (Game|GetPlayerController 0)) "/Game/FirstPerson/Input/IMC_Hovering.IMC_Hovering" 0 "(bIgnoreAllPressedKeysUntilRelease=True,bForceImmediately=False,bNotifyUserSettings=False)")
        (Default|OnInteraction _possibleinteract)))))

(event EventBeginPlay
  (bind _returnvalue (Game|GetPlayerCameraManager 0))
  ;[0 1 0.03071] CAMERA PITCH
  (Variables|/Script/Engine.PlayerCameraManager|SetViewPitchMax _returnvalue (Variables|Default|GetPitch%20Clamp%20Max))
  (Variables|/Script/Engine.PlayerCameraManager|SetViewPitchMin _returnvalue (Variables|Default|GetPitch%20Clamp%20Min))
  (CallFunction|AddFeedbacks))

(event EventTick
  (params (DeltaSeconds :type Float%20%28single-precision%29))
  (Development|SetHiddeninGame (Variables|Character|GetMesh) (< (Default|JPTurboPwr (Variables|Default|GetAC_Jetpack)) 0.2) false))

(event Custom|Landing%20Feedback
  (Camera|PlayWorldCameraShake "/Game/Blueprints/CameraShakes/BP_ShakeLanding.BP_ShakeLanding_C" (Transformation|GetActorLocation) 0.0 5e+02))

(event Custom|StartTurbo
  (bind _rocketright (Variables|Default|GetRocketRight))
  (bind _rocketleft (Variables|Default|GetRocketLeft))
  (Utilities|IsValid (Variables|Niagara|GetRocketDustLeft)
    (:Is%20Not%20Valid
      (Utilities|IsValid (Variables|Niagara|GetRocketDustRight)
        (:Is%20Not%20Valid
          (bind _returnvalue (Niagara|SpawnSystemAttached "/Game/RocketThrusterExhaustFX/FX/NS_RocketExhaust_Plume_2.NS_RocketExhaust_Plume_2" _rocketleft "None" (Variables|/Script/Engine.SceneComponent|GetRelativeLocation _rocketleft) (Variables|/Script/Engine.SceneComponent|GetRelativeRotation _rocketleft) "SnapToTarget" false))
          (Variables|Niagara|SetRocketDustLeft _returnvalue)
          (bind _returnvalue_2 (Niagara|SpawnSystemAttached "/Game/RocketThrusterExhaustFX/FX/NS_RocketExhaust_Plume_2.NS_RocketExhaust_Plume_2" _rocketright "None" (Variables|/Script/Engine.SceneComponent|GetRelativeLocation _rocketright) (Variables|/Script/Engine.SceneComponent|GetRelativeRotation _rocketright) "SnapToTarget" false))
          (Variables|Niagara|SetRocketDustRight _returnvalue_2))))))

(event Custom|AddFeedbacks
  (bind _returnvalue (Game|GetPlayerCharacter 0))
  (bind _returnvalue_2 (Actor|GetComponentbyClass _returnvalue "/Game/FirstPerson/Blueprints/AC_Jetpack.AC_Jetpack_C"))
  (EventDispatchers|BindEventtoOnLanding _returnvalue_2 (delegate Custom|Landing%20Feedback))
  (EventDispatchers|BindEventtoOnStartHovering _returnvalue_2 (delegate Custom|StartTurbo))
  (EventDispatchers|BindEventtoOnStopTurbo _returnvalue_2 (delegate Custom|StopTurbo)))

(event Custom|StopTurbo
  (Utilities|IsValid (Variables|Niagara|GetRocketDustLeft)))

(event Input|EnhancedActionEvents|EnhancedInputActionIA_Move
  (params (ActionValue :type Vector%202D%20Structure) (ElapsedSeconds :type Float%20%28double-precision%29) (TriggeredSeconds :type Float%20%28double-precision%29) (InputAction :type Input%20Action%20Object%20Reference :default "/Game/GameManager/Inputs/IA_Move.IA_Move"))
  (:Started
    (CallFunction|SetMovementCameraFeedbacks)))

(fn ConstructionScript)

(fn SetPossibleInteract
  (params (Interactable :type BP%20Interactable%20Object%20Reference))
  (Variables|Default|SetPossibleInteract Interactable))

(fn SetMovementCameraFeedbacks
  (if (== (Default|JPState (Variables|Default|GetAC_Jetpack)) 0)
    (Camera|PlayWorldCameraShake "/Game/Blueprints/CameraShakes/BP_ShakeStartWalking.BP_ShakeStartWalking_C" (Transformation|GetActorLocation) 0.0 5e+02)))