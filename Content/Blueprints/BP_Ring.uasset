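; A ring checkpoint that the player passes through as one objective in a sequence run by a Ring Manager.
; On overlap it uses a dot product against the collider's up vector to accept only one approach side, then, if it is the current ring, marks itself completed, advances the manager and plays a sound.
; Construction scales the torus by Radius, and a setter toggles the arrow and custom-depth outline.
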(event OnComponentBeginOverlap(Collisions)
  (params (OverlappedComponent :type Primitive%20Component%20Object%20Reference) (OtherActor :type Actor%20Object%20Reference) (OtherComp :type Primitive%20Component%20Object%20Reference) (OtherBodyIndex :type Integer) (bFromSweep :type Boolean) (SweepResult :type Hit%20Result%20Structure%20%28by%20ref%29))
  (bind _ringmanager (Variables|Default|GetringManager))
  ;[0.3882 1 0.8471] Check If The Player Passed Through The Ring
  (if (== OtherActor (Game|GetPlayerCharacter 0))
    (if (> (Math|Vector|DotProduct (- (Transformation|GetActorLocation OtherActor) (Transformation|GetWorldLocation OverlappedComponent)) (Math|Vector|GetUpVector OverlappedComponent)) 0.0)
      ;[1 0.3854 0.3854] Check If We Can Go To The Next Objective
      (Utilities|IsValid _ringmanager
        (:Is%20Valid
          (bind _isthecurrentone (Default|IstheCurrentOne _ringmanager self))
          (if _isthecurrentone
            (Variables|Default|SetisCompleted true)
            (Default|SetupNextObjective _ringmanager)
            (Default|CheckDone _ringmanager)
            (Audio|PlaySound2D "/Game/Assets/Sounds/S_RingValidation.S_RingValidation" 1.0 1.0 0.0 0 0)))
        (:Is%20Not%20Valid
          (Development|PrintString "No assigned to manager" true true "(R=1.000000,G=0.023671,B=0.000000,A=1.000000)"))))))

(event EventBeginPlay
  (Variables|Default|SetisCompleted false))

(fn ConstructionScript
  (bind _radius (Variables|Default|Getradius))
  (bind _sm_torus (Variables|Default|GetSM_Torus))
  (Transformation|SetRelativeScale3D _sm_torus (Math|Vector|MakeVector _radius _radius (.z (Variables|/Script/Engine.SceneComponent|GetRelativeScale3D _sm_torus)))))

(fn GetIsCompleted
  (return (Variables|Default|GetisCompleted)))

(fn SetRingManager
  (params (ringManager :type BP%20Ring%20Manager%20Object%20Reference))
  (Variables|Default|SetringManager ringManager))

(fn SetArrowVisibility
  (params (isVisible :type Boolean))
  (bind _sm_outline (Variables|Default|GetSM_Outline))
  (if isVisible
    (Rendering|SetVisibility (Variables|Default|GetSM_Arrow) true false)
    (Rendering|SetRenderCustomDepth _sm_outline true)
    (else
      (Rendering|SetVisibility (Variables|Default|GetSM_Arrow) false false)
      (Rendering|SetRenderCustomDepth _sm_outline false))))