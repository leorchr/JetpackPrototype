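; BP_JetpackInteractive is the interactive jetpack pickup, which shows the jetpack tutorial text on interaction.
; On BeginPlay it picks a random pitch and yaw once, then loops eased MoveComponentTo calls to bob and tilt its Cube mesh.
; OnInteraction runs the parent logic, then sets the tutorial text through the BP_HUD widget.
; The construction script scales the Cube from AssetScale.
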(event EventBeginPlay
  (bind _maxrotationpitch (Variables|Default|GetMaxRotationPitch))
  (bind _maxrotationpitch_2 (Variables|Default|GetMaxRotationPitch))
  ;[1 1 1] Set a random movement to the pickable objet
  (|CallParentFunction)
  (Variables|Default|SetBasePosition (Variables|/Script/Engine.SceneComponent|GetRelativeLocation (Variables|Default|GetCube)))
  (Variables|Default|SetRandFloatPitch (Math|Random|RandomFloatinRange (- 0.0 _maxrotationpitch_2) _maxrotationpitch_2))
  (Variables|Default|SetRandFloatYaw (Math|Random|RandomFloatinRange (- 0.0 _maxrotationpitch) _maxrotationpitch))
  (Components|MoveComponentTo (Variables|Default|GetCube) (+ (Variables|Default|GetBasePosition) "0.000000,0.000000,50.000000") (Math|Rotator|MakeRotator 0.0 (Variables|Default|GetRandFloatPitch) (Variables|Default|GetRandFloatYaw)) true true (Variables|Default|GetInterpDuration) false :!label _label)
  (Components|MoveComponentTo (Variables|Default|GetCube) (Variables|Default|GetBasePosition) (Math|Rotator|MakeRotator 0.0 (- 0.0 (Variables|Default|GetRandFloatPitch)) (- 0.0 (Variables|Default|GetRandFloatYaw))) true true (Variables|Default|GetInterpDuration) false)
  (goto _label))

(event Collision|EventActorBeginOverlap
  (params (OtherActor :type Actor%20Object%20Reference))
  (|CallParentFunction OtherActor) ; This node is disabled and will not be called.\nDrag off pins to build functionality.
)

(event EventTick
  (params (DeltaSeconds :type Float%20%28single-precision%29))
  (|CallParentFunction DeltaSeconds))

(event EventOnInteraction
  ;[1 1 1] Turn on tuto text of jetpack
  (|CallParentFunction)
  (bind _asbp_hud (Utilities|Casting|CastToBP_HUD (HUD|GetHUD (Game|GetPlayerController 0))))
  (Default|SetJetpackTutoText (Variables|/Game/GameManager/BP_HUD.BP_HUD_C|Getwbp _asbp_hud)))

(fn ConstructionScript
  (|CallParentFunction)
  (Transformation|SetRelativeScale3D (Variables|Default|GetCube) (Math|Conversions|ToVector(Float) (Variables|Default|GetAssetScale))))