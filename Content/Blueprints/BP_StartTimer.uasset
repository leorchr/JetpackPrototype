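; BP_StartTimer is a one-shot trigger volume that starts an on-screen timer when the player character overlaps it.
; It checks the player controller's spaceship component to choose between the spaceship and main HUD widgets.
; It enables that widget's timer, starts it through BP_HUD, then destroys itself.
; The construction script sizes the trigger box from the BoxSize variable.
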(event OnComponentBeginOverlap(TriggerZone)
  (params (OverlappedComponent :type Primitive%20Component%20Object%20Reference) (OtherActor :type Actor%20Object%20Reference) (OtherComp :type Primitive%20Component%20Object%20Reference) (OtherBodyIndex :type Integer) (bFromSweep :type Boolean) (SweepResult :type Hit%20Result%20Structure%20%28by%20ref%29))
  ;[0.5833 1 0.744] Start A Timer
  (if (Variables|/Game/Blueprints/SpaceShip/BP_SpaceShipControllerComponent.BP_SpaceShipControllerComponent_C|GetIsInSpaceShip (Actor|GetComponentbyClass (Game|GetPlayerController 0) "/Game/Blueprints/SpaceShip/BP_SpaceShipControllerComponent.BP_SpaceShipControllerComponent_C"))
    (if (== OtherActor (Game|GetPlayerCharacter 0))
      (bind _asbp_hud (Utilities|Casting|CastToBP_HUD (HUD|GetHUD (Game|GetPlayerController 0))))
      (Default|EnableTimer (Variables|/Game/GameManager/BP_HUD.BP_HUD_C|GetWBPSpaceShip%20Ref _asbp_hud))
      (Default|StartTimerWBPSpaceShip _asbp_hud)
      (Actor|DestroyActor))
    (elif (== OtherActor (Game|GetPlayerCharacter 0))
      (bind _asbp_hud_2 (Utilities|Casting|CastToBP_HUD (HUD|GetHUD (Game|GetPlayerController 0))))
      (Default|EnableTimer (Variables|/Game/GameManager/BP_HUD.BP_HUD_C|GetWBPMain%20Ref _asbp_hud_2))
      (Default|StartTimerWBPMain _asbp_hud_2)
      (Actor|DestroyActor))))

(fn ConstructionScript
  (Components|Box|SetBoxExtent (Variables|Default|GetTriggerZone) (Variables|Default|GetBoxSize) true))