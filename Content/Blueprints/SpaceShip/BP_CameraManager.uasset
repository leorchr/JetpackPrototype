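; Camera manager that changes the spaceship camera's field of view to match first/third-person view and normal/boost mode.
; On BeginPlay it caches the player pawn's camera, sets the first-person FOV and binds to four mode dispatchers on BP_SpaceShipController.
; Each handler only sets a target FOV.
; Tick eases the camera toward that target with a delta-time-scaled Lerp.
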(event Custom|FPS_BoostMode_Event
  (Utilities|IsValid (Variables|Default|GetCameraPawn)
    (:Is%20Valid
      (Variables|FOV|SetCurrentFOV (Variables|FOV|GetFOV_FirstPersonNitro)))))

(event Custom|TPS_BoostMode_Event
  (Utilities|IsValid (Variables|Default|GetCameraPawn)
    (:Is%20Valid
      (Variables|FOV|SetCurrentFOV (Variables|FOV|GetFOV_ThirdPersonNitro)))))

(event Custom|FPS_NormalMode_Event
  (Utilities|IsValid (Variables|Default|GetCameraPawn)
    (:Is%20Valid
      (Variables|FOV|SetCurrentFOV (Variables|FOV|GetFOV_FirstPerson)))))

(event Custom|TPS_NormalMode_Event
  (Utilities|IsValid (Variables|Default|GetCameraPawn)
    (:Is%20Valid
      (Variables|FOV|SetCurrentFOV (Variables|FOV|GetFOV_ThirdPerson)))))

(event EventBeginPlay
  (bind _asbp_space_ship_controller (Utilities|Casting|CastToBP_SpaceShipController (Game|GetPlayerController 0)))
  (Utilities|IsValid _asbp_space_ship_controller
    (:Is%20Valid
      (Variables|Components|SetBP_Space_Ship_Controller _asbp_space_ship_controller)
      (bind _asbp_space_ship_pawn (Utilities|Casting|CastToBP_SpaceShipPawn (Game|Player|GetPlayerPawn 0)))
      (bind _output_get (Variables|Default|SetCameraPawn (Variables|/Game/Blueprints/SpaceShip/BP_SpaceShipPawn.BP_SpaceShipPawn_C|GetCamera _asbp_space_ship_pawn)))
      (Utilities|IsValid _output_get
        (:Is%20Valid
          (Camera|SetFieldOfView _output_get (Variables|FOV|GetFOV_FirstPerson))
          (EventDispatchers|AssignFPSBoostMode (Variables|Components|GetBP_Space_Ship_Controller) (delegate Custom|FPS_BoostMode_Event))
          (EventDispatchers|AssignFPSNormalMode (Variables|Components|GetBP_Space_Ship_Controller) (delegate Custom|FPS_NormalMode_Event))
          (EventDispatchers|AssignTPSNormalMode (Variables|Components|GetBP_Space_Ship_Controller) (delegate Custom|TPS_NormalMode_Event))
          (EventDispatchers|AssignTPSBoostMode (Variables|Components|GetBP_Space_Ship_Controller) (delegate Custom|TPS_BoostMode_Event)))))))

(event EventTick
  (params (DeltaSeconds :type Float%20%28single-precision%29))
  (if (!= (Variables|/Script/Engine.CameraComponent|GetFieldOfView (Variables|Default|GetCameraPawn)) (Variables|FOV|GetCurrentFOV))
    (Camera|SetFieldOfView (Variables|Default|GetCameraPawn) (Math|Float|Lerp (Variables|/Script/Engine.CameraComponent|GetFieldOfView (Variables|Default|GetCameraPawn)) (Variables|FOV|GetCurrentFOV) (* DeltaSeconds (Variables|Default|GetFOV_Speed))))))

(fn ConstructionScript)