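; Spaceship pawn that the player character can board and leave, with first-person, third-person and boost camera views.
; ControlTrigger overlaps toggle a prompt widget and register or clear the ship as the character's interactable.
; StartInteraction possesses the ship, hides and attaches the driver, and binds camera events to BP_SpaceShipControllerComponent's mode dispatchers.
; IA_Interact hands possession back to the driver and restores its visibility and collision.
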(event OnComponentBeginOverlap(ControlTrigger)
  (params (OverlappedComponent :type Primitive%20Component%20Object%20Reference) (OtherActor :type Actor%20Object%20Reference) (OtherComp :type Primitive%20Component%20Object%20Reference) (OtherBodyIndex :type Integer) (bFromSweep :type Boolean) (SweepResult :type Hit%20Result%20Structure%20%28by%20ref%29))
  ;[0 1 0.1794] Player enter collision
  (if (not (Pawn|IsPlayerControlled self))
    (bind _yes (Class|BPICharacter|IsPlayer(Message) OtherActor))
    (if _yes
      (CallFunction|ToggleInstructionWidget true)
      (Class|BPICharacter|SetInteractable(Message) OtherActor self))))

(event OnComponentEndOverlap(ControlTrigger)
  (params (OverlappedComponent :type Primitive%20Component%20Object%20Reference) (OtherActor :type Actor%20Object%20Reference) (OtherComp :type Primitive%20Component%20Object%20Reference) (OtherBodyIndex :type Integer))
  ;[1 0 0] Player exit collision
  (if (not (Pawn|IsPlayerControlled self))
    (bind _yes (Class|BPICharacter|IsPlayer(Message) OtherActor))
    (if _yes
      (CallFunction|ToggleInstructionWidget false)
      (Class|BPICharacter|SetInteractable(Message) OtherActor))))

(event Custom|SetThirdPerson
  (bind _springarm (Variables|Default|GetSpringArm))
  ;[0.9384 0.4679 1] Base
  (Rendering|SetVisibility (Variables|Default|GetStaticMesh) true false)
  (Variables|/Script/Engine.SpringArmComponent|SetTargetArmLength _springarm 1e+03)
  (Variables|/Script/Engine.SpringArmComponent|SetSocketOffset _springarm (Math|Vector|MakeVector 0.0 0.0 1e+03))
  (Transformation|SetRelativeRotation (Variables|Default|GetCamera) (Math|Rotator|MakeRotator 0.0 -1e+01 0.0) false false))

(event Custom|SetFirstPerson
  (bind _springarm (Variables|Default|GetSpringArm))
  ;[0.9384 0.4679 1] Base
  (Rendering|SetVisibility (Variables|Default|GetStaticMesh) false false)
  (Variables|/Script/Engine.SpringArmComponent|SetTargetArmLength _springarm 0.0)
  (Variables|/Script/Engine.SpringArmComponent|SetSocketOffset _springarm (Math|Vector|MakeVector 0.0 0.0 0.0))
  (Transformation|SetRelativeRotation (Variables|Default|GetCamera) (Math|Rotator|MakeRotator 0.0 0.0 0.0) false false))

(event Custom|TPS_BoostMode_Event
  (bind _springarm (Variables|Default|GetSpringArm))
  (Rendering|SetVisibility (Variables|Default|GetStaticMesh) true false)
  (Variables|/Script/Engine.SpringArmComponent|SetTargetArmLength _springarm 8e+02)
  (Variables|/Script/Engine.SpringArmComponent|SetSocketOffset _springarm (Math|Vector|MakeVector 0.0 0.0 8.5e+02))
  (Transformation|SetRelativeRotation (Variables|Default|GetCamera) (Math|Rotator|MakeRotator 0.0 -1e+01 0.0) false false))

(event Input|EnhancedActionEvents|EnhancedInputActionIA_Interact
  (params (ActionValue :type Boolean) (ElapsedSeconds :type Float%20%28double-precision%29) (TriggeredSeconds :type Float%20%28double-precision%29) (InputAction :type Input%20Action%20Object%20Reference :default "/Game/GameManager/Inputs/IA_Interact.IA_Interact"))
  ;[0.5167 1 0.701] Interact input
  (:Started
    (bind _driver (Variables|Default|GetDriver)
      (:then
        (Collision|SetActorEnableCollision _driver true)
        (Pawn|Possess (Game|GetPlayerController 0) _driver)
        ;;[0 1 0.026] Enable Mesh, Collision, Shadow
        (Rendering|SetActorHiddenInGame _driver false)
        (Collision|SetCollisionEnabled (Variables|/Script/Engine.Character|GetCapsuleComponent _driver) "QueryAndPhysics")
        (Rendering|SetCastShadow (Variables|/Script/Engine.Character|GetMesh _driver) true)
        (Variables|/Game/Blueprints/SpaceShip/BP_SpaceShipControllerComponent.BP_SpaceShipControllerComponent_C|SetIsInSpaceShip (Actor|GetComponentbyClass (Game|GetPlayerController 0) "/Game/Blueprints/SpaceShip/BP_SpaceShipControllerComponent.BP_SpaceShipControllerComponent_C") false)
        (CallFunction|SetThirdPerson))
      (:else))))

(event EventStartInteraction
  (params (InteractingCharacter :type Character%20Object%20Reference))
  (bind _returnvalue (Game|GetPlayerController 0))
  (bind _returnvalue_2 (Actor|GetComponentbyClass _returnvalue "/Game/Blueprints/SpaceShip/BP_SpaceShipControllerComponent.BP_SpaceShipControllerComponent_C"))
  ;[0.1498 0.9003 1] Start Interaction
  (Variables|Default|SetDriver InteractingCharacter)
  (Pawn|Possess (Game|GetPlayerController 0) self)
  (CallFunction|ToggleInstructionWidget false)
  (Collision|SetActorEnableCollision (Variables|Default|GetDriver) false)
  (Transformation|AttachComponentToComponent (Variables|Default|GetDriver) (Variables|Default|GetControlTrigger) "None" "KeepWorld" "KeepWorld" "KeepWorld" true)
  ;;[1 0 0] Disable Mesh, Collision, Shadow
  (Rendering|SetActorHiddenInGame (Variables|Default|GetDriver) true)
  (Collision|SetCollisionEnabled (Variables|/Script/Engine.Character|GetCapsuleComponent (Variables|Default|GetDriver)) "NoCollision")
  (Rendering|SetCastShadow (Variables|/Script/Engine.Character|GetMesh (Variables|Default|GetDriver)) false)
  (Variables|/Game/Blueprints/SpaceShip/BP_SpaceShipControllerComponent.BP_SpaceShipControllerComponent_C|SetIsInSpaceShip (Actor|GetComponentbyClass (Game|GetPlayerController 0) "/Game/Blueprints/SpaceShip/BP_SpaceShipControllerComponent.BP_SpaceShipControllerComponent_C") true)
  (CallFunction|SetFirstPerson)
  (Default|ControllerBegin _returnvalue_2)
  (bind _output_get (Variables|Components|SetBP_Space_Ship_Controller _returnvalue_2))
  (EventDispatchers|BindEventtoFPSNormalMode _output_get (delegate Custom|SetFirstPerson))
  (EventDispatchers|BindEventtoTPSNormalMode _output_get (delegate Custom|SetThirdPerson))
  (Variables|/Script/Engine.SpringArmComponent|SetTargetArmLength (Variables|Default|GetSpringArm) 0.0)
  (EventDispatchers|BindEventtoTPSBoostMode _output_get (delegate Custom|TPS_BoostMode_Event)))

(fn ConstructionScript)

(fn ToggleInstructionWidget
  (params (Show%20/Hide :type Boolean))
  (if Show%20/Hide
    (Variables|Default|GetWdgInstruction
      (:then
        _)
      (:else
        (bind _returnvalue (UserInterface|CreateWidget "/Game/Character/Interfaces/W_SpaceshipInteract.W_SpaceshipInteract_C" (Game|GetPlayerController 0)))
        (Variables|Default|SetWdgInstruction _returnvalue)))
    (UserInterface|Viewport|AddtoViewport (Variables|Default|GetWdgInstruction) 0)
    (else
      (bind _wdginstruction (Variables|Default|GetWdgInstruction)
        (:then
          (if (UserInterface|Viewport|IsinViewport _wdginstruction)
            (Widget|RemovefromParent _wdginstruction)))
        (:else)))))