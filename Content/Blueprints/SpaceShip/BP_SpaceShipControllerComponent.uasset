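; Player controller component that flies the spaceship pawn, constantly pushing it along its camera's forward vector.
; Stick input drives pitch and yaw with interpolated banking of the control rotation, plus the mesh in third person, levelling out on release.
; Analog boost scales speed and drains a timed nitro reserve that recharges afterward, locking until full if emptied.
; View switching and boost trigger matching first- or third-person mode calls.
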(event Custom|Controller%20Begin
  ;[0.2268 0 1] Setup Variables
  (Variables|Default|SetCurrentViewMode "NewEnumerator0")
  (Variables|Speed|SetCurrentSpeed (Variables|Speed|GetSpeed))
  (bind _asbp_space_ship_pawn (Utilities|Casting|CastToBP_SpaceShipPawn (Game|Player|GetPlayerPawn 0)))
  (Utilities|IsValid _asbp_space_ship_pawn
    (:Is%20Valid
      (Variables|Components|SetSpaceShipPawn _asbp_space_ship_pawn)
      (Utilities|IsValid (Variables|/Game/Blueprints/SpaceShip/BP_SpaceShipPawn.BP_SpaceShipPawn_C|GetFloatingPawnMovement _asbp_space_ship_pawn)
        (:Is%20Valid
          (Variables|Default|SetFloatingPawnMovement (Variables|/Game/Blueprints/SpaceShip/BP_SpaceShipPawn.BP_SpaceShipPawn_C|GetFloatingPawnMovement _asbp_space_ship_pawn))
          (Variables|/Script/Engine.FloatingPawnMovement|SetMaxSpeed (Variables|Default|GetFloatingPawnMovement) (Variables|Speed|GetSpeed))
          (bind _asbp_player_controller (Utilities|Casting|CastToBP_PlayerController (Game|GetPlayerController 0)))
          (Variables|Components|SetBP_Player_Controller _asbp_player_controller))))))

(event Input|EnhancedActionEvents|EnhancedInputActionIA_MoveAndLook
  (params (ActionValue :type Vector%202D%20Structure) (ElapsedSeconds :type Float%20%28double-precision%29) (TriggeredSeconds :type Float%20%28double-precision%29) (InputAction :type Input%20Action%20Object%20Reference :default "/Game/GameManager/Inputs/IA_MoveAndLook.IA_MoveAndLook"))
  (bind _returnvalue (Game|GetPlayerController 0))
  (bind _returnvalue_2 (Math|Conversions|ToVector(Vector2D) ActionValue))
  (bind _spaceshippawn (Variables|Components|GetSpaceShipPawn))
  (bind _spaceshippawn_2 (Variables|Components|GetSpaceShipPawn))
  (bind _returnvalue_3 (Math|Vector|VectorClampSizeMax _returnvalue_2 1.0))
  (bind _returnvalue_4 (Transformation|GetActorRotation _spaceshippawn))
  (bind _staticmesh (Variables|/Game/Blueprints/SpaceShip/BP_SpaceShipPawn.BP_SpaceShipPawn_C|GetStaticMesh _spaceshippawn_2))
  (bind _relativerotation (Variables|/Script/Engine.SceneComponent|GetRelativeRotation _staticmesh))
  ;[0 1 0.2822] Left Joystick pitch and yaw movements
  (:Triggered
    (Class|PlayerController|AddPitchInput _returnvalue (* (Variables|Movements|GetSensitivity) (.y _returnvalue_3)))
    (Class|PlayerController|AddYawInput _returnvalue (* (Variables|Movements|GetSensitivity) (.x _returnvalue_3)))
    (Variables|ActorRotation|SetCurrentActorRollDegree (* (.x _returnvalue_3) (Variables|ActorRotation|GetMaxActorRollDegree)))
    (Variables|MeshRotation|SetCurrentMeshRollDegree (* (.x _returnvalue_3) (Variables|MeshRotation|GetMaxMeshRollDegree)))
    (if (!= (.x _returnvalue_3) 0.0)
      ;[1 0 0.807] Actor Roll Left/Right
      (Pawn|SetControlRotation (Game|GetPlayerController 0) (Math|Interpolation|RInterpTo (Math|Rotator|MakeRotator (.roll _returnvalue_4) (.pitch _returnvalue_4) (.yaw _returnvalue_4)) (Math|Rotator|MakeRotator (Variables|ActorRotation|GetCurrentActorRollDegree) (.pitch _returnvalue_4) (.yaw _returnvalue_4)) (Utilities|Time|GetWorldDeltaSeconds) (Variables|ActorRotation|GetResetActorRollInterpSpeed)))
      ;[1 0.2423 0] Spaceship Rotation in third person
      (if (Utilities|Enum|Equal(Enum) (Variables|Default|GetCurrentViewMode) "NewEnumerator1")
        (Transformation|SetRelativeRotation _staticmesh (Math|Interpolation|RInterpTo (Math|Rotator|MakeRotator (.roll _relativerotation) (.pitch _relativerotation) (.yaw _relativerotation)) (Math|Rotator|MakeRotator (Variables|MeshRotation|GetCurrentMeshRollDegree) (.pitch _relativerotation) (.yaw _relativerotation)) (Utilities|Time|GetWorldDeltaSeconds) (Variables|MeshRotation|GetResetMeshRollInterpSpeed)) false false))))
  (:Started
    (Variables|ActorRotation|SetResetRoll false))
  (:Canceled
    (Variables|ActorRotation|SetResetRoll true :!label _label))
  (:Completed
    (goto _label)))

(event Input|EnhancedActionEvents|EnhancedInputActionIA_SwitchViewMode
  (params (ActionValue :type Boolean) (ElapsedSeconds :type Float%20%28double-precision%29) (TriggeredSeconds :type Float%20%28double-precision%29) (InputAction :type Input%20Action%20Object%20Reference :default "/Game/GameManager/Inputs/IA_SwitchViewMode.IA_SwitchViewMode"))
  ;[0.3551 0 1] Switch First/Third Person
  (:Started
    (switch Utilities|FlowControl|Switch|SwitchonE_ViewMode (Variables|Default|GetCurrentViewMode)
      (:NewEnumerator0
        (Variables|Default|SetCurrentViewMode "NewEnumerator1")
        (Default|CallTPSNormalMode))
      (:NewEnumerator1
        (Variables|Default|SetCurrentViewMode "NewEnumerator0")
        (Default|CallFPSNormalMode)))))

(event Input|EnhancedActionEvents|EnhancedInputActionIA_Boost
  (params (ActionValue :type Float%20%28double-precision%29) (ElapsedSeconds :type Float%20%28double-precision%29) (TriggeredSeconds :type Float%20%28double-precision%29) (InputAction :type Input%20Action%20Object%20Reference :default "/Game/GameManager/Inputs/IA_Boost.IA_Boost"))
  ;[1 0.375 0.4155] Boost Mode
  (:Triggered
    ;;[0.1928 0 1] Start Boost if the player have boost
    (if (and (not (Variables|Speed|GetWaitForSeconds)) (> (Variables|Speed|GetBoostDuration) 0.0))
      (Utilities|FlowControl|Sequence
        (:then_0
          ;;[0 0.7125 1] Adjust current boost speed based on button press intensity
          (bind _output_get (Variables|Speed|SetCurrentSpeed (+ (Variables|Speed|GetSpeed) (* ActionValue (- (Variables|Speed|GetNitroSpeed) (Variables|Speed|GetSpeed))))))
          (Variables|/Script/Engine.FloatingPawnMovement|SetMaxSpeed (Variables|Default|GetFloatingPawnMovement) _output_get)
          ;;[1 0.3485 0] Decrease boost time left
          (Variables|Speed|SetBoostDuration (- (Variables|Speed|GetBoostDuration) (Utilities|Time|GetWorldDeltaSeconds)))
          (if (< (Variables|Speed|GetBoostDuration) 0.0)
            (CallFunction|StopInput)))
        (:then_1
          ;;[1 0 0.7379] Start Boost Mode
          (if (Variables|Speed|GetOnlyOnce)
            (Variables|Speed|SetOnlyOnce false)
            (Variables|Speed|SetCurrentNitroState "NewEnumerator1")
            (switch Utilities|FlowControl|Switch|SwitchonE_ViewMode (Variables|Default|GetCurrentViewMode)
              (:NewEnumerator0
                (Default|CallFPSBoostMode))
              (:NewEnumerator1
                (Default|CallTPSBoostMode))))))))
  (:Completed
    ;;[1 0 0.03236] Reset values at the end of the boost
    (Utilities|FlowControl|Sequence
      (:then_0
        (bind _output_get_2 (Variables|Speed|SetCurrentSpeed (Variables|Speed|GetSpeed)))
        (Variables|/Script/Engine.FloatingPawnMovement|SetMaxSpeed (Variables|Default|GetFloatingPawnMovement) _output_get_2)
        (switch Utilities|FlowControl|Switch|SwitchonE_ViewMode (Variables|Default|GetCurrentViewMode)
          (:NewEnumerator0
            (Default|CallFPSNormalMode))
          (:NewEnumerator1
            (Default|CallTPSNormalMode))))
      (:then_1
        (Variables|Speed|SetOnlyOnce true)
        (Variables|Speed|SetCurrentNitroState "NewEnumerator2")))))

(event EventTick
  (params (DeltaSeconds :type Float%20%28single-precision%29))
  (bind _returnvalue (Game|GetPlayerController 0))
  (bind _spaceshippawn (Variables|Components|GetSpaceShipPawn))
  (bind _spaceshippawn_2 (Variables|Components|GetSpaceShipPawn))
  (bind _spaceshippawn_3 (Variables|Components|GetSpaceShipPawn))
  (bind _bp_player_controller (Variables|Components|GetBP_Player_Controller))
  (bind _returnvalue_2 (Transformation|GetActorRotation _spaceshippawn_2))
  (bind _staticmesh (Variables|/Game/Blueprints/SpaceShip/BP_SpaceShipPawn.BP_SpaceShipPawn_C|GetStaticMesh _spaceshippawn))
  (bind _relativerotation (Variables|/Script/Engine.SceneComponent|GetRelativeRotation _staticmesh))
  ;[0 1 0.5608] Always going forward
  (Utilities|IsValid _bp_player_controller
    (:Is%20Valid
      (if (Utilities|Enum|Equal(Enum) (Variables|/Game/GameManager/BP_PlayerController.BP_PlayerController_C|GetPawnPossessed _bp_player_controller) "NewEnumerator1")
        (Utilities|FlowControl|Sequence
          (:then_0
            (Utilities|IsValid _spaceshippawn_3
              (:Is%20Valid
                (Class|PawnMovementComponent|AddInputVector (Variables|Default|GetFloatingPawnMovement) (* (Math|Vector|GetForwardVector (Variables|/Game/Blueprints/SpaceShip/BP_SpaceShipPawn.BP_SpaceShipPawn_C|GetCamera _spaceshippawn_3)) (Variables|Speed|GetCurrentSpeed)) false)
                ;[1 0 0.807] Reset Actor Roll if no input
                (if (Variables|ActorRotation|GetResetRoll)
                  (Utilities|FlowControl|Sequence
                    (:then_0
                      (if (!= (.roll (Transformation|GetActorRotation (Game|GetPlayerController 0))) 0.0)
                        (Pawn|SetControlRotation (Game|GetPlayerController 0) (Math|Interpolation|RInterpTo (Math|Rotator|MakeRotator (.roll _returnvalue_2) (.pitch _returnvalue_2) (.yaw _returnvalue_2)) (Math|Rotator|MakeRotator 0.0 (.pitch _returnvalue_2) (.yaw _returnvalue_2)) (Utilities|Time|GetWorldDeltaSeconds) (Variables|ActorRotation|GetResetActorRollInterpSpeed)))))
                    (:then_1
                      ;[1 0.2423 0] Reset Meshs Roll if no input
                      (if (!= (.roll (Variables|/Script/Engine.SceneComponent|GetRelativeRotation _staticmesh)) 0.0)
                        (Transformation|SetRelativeRotation _staticmesh (Math|Interpolation|RInterpTo (Math|Rotator|MakeRotator (.roll _relativerotation) (.pitch _relativerotation) (.yaw _relativerotation)) (Math|Rotator|MakeRotator 0.0 (.pitch _relativerotation) (.yaw _relativerotation)) (Utilities|Time|GetWorldDeltaSeconds) (Variables|MeshRotation|GetResetMeshRollInterpSpeed)) false false))))))))
          (:then_1
            ;[0 0.9377 1] Recharge Nitro
            (if (and (Utilities|Enum|Equal(Enum) (Variables|Speed|GetCurrentNitroState) "NewEnumerator2") (< (Variables|Speed|GetBoostDuration) (Variables|Speed|GetBoostBaseDuration)))
              (Variables|Speed|SetBoostDuration (+ (Variables|Speed|GetBoostDuration) DeltaSeconds))
              (else
                (Variables|Speed|SetWaitForSeconds false)))))
        (else
          (Transformation|SetActorRotation _returnvalue (Math|Rotator|MakeRotator 0.0 0.0 (.yaw (Camera|GetCameraRotation (Variables|/Script/Engine.PlayerController|GetPlayerCameraManager _returnvalue))))))))))

(fn StopInput
  (Utilities|FlowControl|Sequence
    (:then_0
      ;[0.8579 0 1] Reset Speed
      (bind _output_get (Variables|Speed|SetCurrentSpeed (Variables|Speed|GetSpeed)))
      (Variables|/Script/Engine.FloatingPawnMovement|SetMaxSpeed (Variables|Default|GetFloatingPawnMovement) _output_get)
      (switch Utilities|FlowControl|Switch|SwitchonE_ViewMode (Variables|Default|GetCurrentViewMode)
        (:NewEnumerator0
          (Default|CallFPSNormalMode))
        (:NewEnumerator1
          (Default|CallTPSNormalMode))))
    (:then_1
      ;[0 0.4357 1] Cancel input
      (Variables|Speed|SetWaitForSeconds true))
    (:then_2
      ;[0.4097 1 0] Start Recharging boost
      (Variables|Speed|SetCurrentNitroState "NewEnumerator2"))))