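; Player controller for a spaceship that constantly flies forward along the pawn camera's direction.
; Enhanced Input drives pitch and yaw, boost scales speed toward nitro, and a toggle switches first and third person, calling matching normal or boost mode functions.
; Steering interpolates banking roll on the control rotation, plus the mesh in third person; Tick eases both level when input stops.
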(event Input|EnhancedActionEvents|EnhancedInputActionIA_MoveAndLook
  (params (ActionValue :type Vector%202D%20Structure) (ElapsedSeconds :type Float%20%28double-precision%29) (TriggeredSeconds :type Float%20%28double-precision%29) (InputAction :type Input%20Action%20Object%20Reference :default "/Game/GameManager/Inputs/IA_MoveAndLook.IA_MoveAndLook"))
  (bind _returnvalue (Math|Conversions|ToVector(Vector2D) ActionValue))
  (bind _spaceshippawn (Variables|References|GetSpaceShipPawn))
  (bind _spaceshippawn_2 (Variables|References|GetSpaceShipPawn))
  (bind _returnvalue_2 (Math|Vector|VectorClampSizeMax _returnvalue 1.0))
  (bind _returnvalue_3 (Transformation|GetActorRotation _spaceshippawn))
  (bind _staticmesh (Variables|/Game/Blueprints/SpaceShip/BP_SpaceShipPawn.BP_SpaceShipPawn_C|GetStaticMesh _spaceshippawn_2))
  (bind _relativerotation (Variables|/Script/Engine.SceneComponent|GetRelativeRotation _staticmesh))
  ;[0 1 0.2822] Left Joystick pitch and yaw movements
  (:Triggered
    (Class|PlayerController|AddPitchInput self (* (Variables|Movement|GetSensitivity) (.y _returnvalue_2)))
    (Class|PlayerController|AddYawInput self (* (Variables|Movement|GetSensitivity) (.x _returnvalue_2)))
    (Variables|ActorRotation|SetCurrentActorRollDegree (* (.x _returnvalue_2) (Variables|ActorRotation|GetMaxActorRollDegree)))
    (Variables|MeshRotation|SetCurrentMeshRollDegree (* (.x _returnvalue_2) (Variables|MeshRotation|GetMaxMeshRollDegree)))
    (if (!= (.x _returnvalue_2) 0.0)
      ;[1 0 0.807] Actor Roll Left/Right
      (Pawn|SetControlRotation (Math|Interpolation|RInterpTo (Math|Rotator|MakeRotator (.roll _returnvalue_3) (.pitch _returnvalue_3) (.yaw _returnvalue_3)) (Math|Rotator|MakeRotator (Variables|ActorRotation|GetCurrentActorRollDegree) (.pitch _returnvalue_3) (.yaw _returnvalue_3)) (Utilities|Time|GetWorldDeltaSeconds) (Variables|ActorRotation|GetResetActorRollInterpSpeed)))
      ;[1 0.2423 0] Spaceship Rotation in third person
      (if (Utilities|Enum|Equal(Enum) (Variables|Default|GetCurrentViewMode) "NewEnumerator1")
        (Transformation|SetRelativeRotation _staticmesh (Math|Interpolation|RInterpTo (Math|Rotator|MakeRotator (.roll _relativerotation) (.pitch _relativerotation) (.yaw _relativerotation)) (Math|Rotator|MakeRotator (Variables|MeshRotation|GetCurrentMeshRollDegree) (.pitch _relativerotation) (.yaw _relativerotation)) (Utilities|Time|GetWorldDeltaSeconds) (Variables|MeshRotation|GetResetMeshRollInterpSpeed)) false false))))
  (:Started
    (Variables|ActorRotation|SetResetRoll false))
  (:Canceled
    (Variables|ActorRotation|SetResetRoll true :!label _label))
  (:Completed
    (goto _label)))

(event Input|EnhancedActionEvents|EnhancedInputActionIA_SwitchViewMode
  (params (ActionValue :type Boolean) (ElapsedSeconds :type Float%20%28double-precision%29) (TriggeredSeconds :type Float%20%28double-precision%29) (InputAction :type Input%20Action%20Object%20Reference :default "/Game/GameManager/Inputs/IA_SwitchViewMode.IA_SwitchViewMode"))
  ;[0.3551 0 1] Switch First/Third Person
  (:Started
    (switch Utilities|FlowControl|Switch|SwitchonE_ViewMode (Variables|Default|GetCurrentViewMode)
      (:NewEnumerator0
        (Variables|Default|SetCurrentViewMode "NewEnumerator1")
        (Default|CallTPSNormalMode))
      (:NewEnumerator1
        (Variables|Default|SetCurrentViewMode "NewEnumerator0")
        (Default|CallFPSNormalMode)))))

(event Input|EnhancedActionEvents|EnhancedInputActionIA_Boost
  (params (ActionValue :type Float%20%28double-precision%29) (ElapsedSeconds :type Float%20%28double-precision%29) (TriggeredSeconds :type Float%20%28double-precision%29) (InputAction :type Input%20Action%20Object%20Reference :default "/Game/GameManager/Inputs/IA_Boost.IA_Boost"))
  ;[1 0 0.06486] Boost Mode
  (:Triggered
    (bind _output_get (Variables|Speed|SetCurrentSpeed (+ (Variables|Speed|GetSpeed) (* ActionValue (- (Variables|Speed|GetNitroSpeed) (Variables|Speed|GetSpeed))))))
    (Variables|/Script/Engine.FloatingPawnMovement|SetMaxSpeed (Variables|Default|GetFloatingPawnMovement) _output_get))
  (:Started
    (switch Utilities|FlowControl|Switch|SwitchonE_ViewMode (Variables|Default|GetCurrentViewMode)
      (:NewEnumerator0
        (Default|CallFPSBoostMode))
      (:NewEnumerator1
        (Default|CallTPSBoostMode))))
  (:Canceled
    (bind _output_get_2 (Variables|Speed|SetCurrentSpeed (Variables|Speed|GetSpeed) :!label _label))
    (Variables|/Script/Engine.FloatingPawnMovement|SetMaxSpeed (Variables|Default|GetFloatingPawnMovement) _output_get_2)
    (switch Utilities|FlowControl|Switch|SwitchonE_ViewMode (Variables|Default|GetCurrentViewMode)
      (:NewEnumerator0
        (Default|CallFPSNormalMode))
      (:NewEnumerator1
        (Default|CallTPSNormalMode))))
  (:Completed
    (goto _label)))

(event EventBeginPlay
  ;[0.2268 0 1] Setup Variables
  (Input|AddMappingContext (PlayerController|LocalPlayerSubsystems|GetEnhancedInputLocalPlayerSubsystem) "/Game/GameManager/Inputs/IMC_SpaceShip.IMC_SpaceShip" 0 "(bIgnoreAllPressedKeysUntilRelease=True,bForceImmediately=False,bNotifyUserSettings=False)")
  (Variables|Default|SetCurrentViewMode "NewEnumerator0")
  (Variables|Speed|SetCurrentSpeed (Variables|Speed|GetSpeed))
  (bind _asbp_space_ship_pawn (Utilities|Casting|CastToBP_SpaceShipPawn (Game|Player|GetPlayerPawn 0)))
  (Utilities|IsValid _asbp_space_ship_pawn
    (:Is%20Valid
      (Variables|References|SetSpaceShipPawn _asbp_space_ship_pawn)
      (Utilities|IsValid (Variables|/Game/Blueprints/SpaceShip/BP_SpaceShipPawn.BP_SpaceShipPawn_C|GetFloatingPawnMovement _asbp_space_ship_pawn)
        (:Is%20Valid
          (Variables|Default|SetFloatingPawnMovement (Variables|/Game/Blueprints/SpaceShip/BP_SpaceShipPawn.BP_SpaceShipPawn_C|GetFloatingPawnMovement _asbp_space_ship_pawn))
          (Variables|/Script/Engine.FloatingPawnMovement|SetMaxSpeed (Variables|Default|GetFloatingPawnMovement) (Variables|Speed|GetSpeed)))))))

(event EventTick
  (params (DeltaSeconds :type Float%20%28single-precision%29))
  (bind _spaceshippawn (Variables|References|GetSpaceShipPawn))
  (bind _spaceshippawn_2 (Variables|References|GetSpaceShipPawn))
  (bind _spaceshippawn_3 (Variables|References|GetSpaceShipPawn))
  (bind _returnvalue (Transformation|GetActorRotation _spaceshippawn_2))
  (bind _staticmesh (Variables|/Game/Blueprints/SpaceShip/BP_SpaceShipPawn.BP_SpaceShipPawn_C|GetStaticMesh _spaceshippawn))
  (bind _relativerotation (Variables|/Script/Engine.SceneComponent|GetRelativeRotation _staticmesh))
  ;[0 1 0.5608] Always going forward
  (Utilities|IsValid _spaceshippawn_3
    (:Is%20Valid
      (Class|PawnMovementComponent|AddInputVector (Variables|Default|GetFloatingPawnMovement) (* (Math|Vector|GetForwardVector (Variables|/Game/Blueprints/SpaceShip/BP_SpaceShipPawn.BP_SpaceShipPawn_C|GetCamera _spaceshippawn_3)) (Variables|Speed|GetCurrentSpeed)) false)
      ;[1 0 0.807] Reset Actor Roll if no input
      (if (Variables|ActorRotation|GetResetRoll)
        (Utilities|FlowControl|Sequence
          (:then_0
            (if (!= (.roll (Transformation|GetActorRotation)) 0.0)
              (Pawn|SetControlRotation (Math|Interpolation|RInterpTo (Math|Rotator|MakeRotator (.roll _returnvalue) (.pitch _returnvalue) (.yaw _returnvalue)) (Math|Rotator|MakeRotator 0.0 (.pitch _returnvalue) (.yaw _returnvalue)) (Utilities|Time|GetWorldDeltaSeconds) (Variables|ActorRotation|GetResetActorRollInterpSpeed)))))
          (:then_1
            ;[1 0.2423 0] Reset Meshs Roll if no input
            (if (!= (.roll (Variables|/Script/Engine.SceneComponent|GetRelativeRotation _staticmesh)) 0.0)
              (Transformation|SetRelativeRotation _staticmesh (Math|Interpolation|RInterpTo (Math|Rotator|MakeRotator (.roll _relativerotation) (.pitch _relativerotation) (.yaw _relativerotation)) (Math|Rotator|MakeRotator 0.0 (.pitch _relativerotation) (.yaw _relativerotation)) (Utilities|Time|GetWorldDeltaSeconds) (Variables|MeshRotation|GetResetMeshRollInterpSpeed)) false false))))))))

(fn ConstructionScript)