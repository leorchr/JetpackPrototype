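; Base interactable actor that the player can use when inside its pickup sphere.
; The construction script sizes the sphere from PickupRadius, and BeginPlay caches the HUD widget from BP_HUD.
; Sphere overlaps with the player set or clear the character's possible interaction and show or hide the prompt.
; OnInteraction destroys the actor and hides the prompt.
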(event OnComponentBeginOverlap(Sphere)
  (params (OverlappedComponent :type Primitive%20Component%20Object%20Reference) (OtherActor :type Actor%20Object%20Reference) (OtherComp :type Primitive%20Component%20Object%20Reference) (OtherBodyIndex :type Integer) (bFromSweep :type Boolean) (SweepResult :type Hit%20Result%20Structure%20%28by%20ref%29))
  (bind _wbp (Variables|Default|Getwbp))
  (if (== OtherActor (Game|GetPlayerCharacter 0))
    (Default|SetPossibleInteract (.AsBP%20Character (Utilities|Casting|CastToBP_Character OtherActor)) self)
    (Utilities|IsValid _wbp
      (:Is%20Valid
        (Default|ShowInteraction _wbp)))))

(event OnComponentEndOverlap(Sphere)
  (params (OverlappedComponent :type Primitive%20Component%20Object%20Reference) (OtherActor :type Actor%20Object%20Reference) (OtherComp :type Primitive%20Component%20Object%20Reference) (OtherBodyIndex :type Integer))
  (bind _wbp (Variables|Default|Getwbp))
  (if (== OtherActor (Game|GetPlayerCharacter 0))
    (Default|SetPossibleInteract (.AsBP%20Character (Utilities|Casting|CastToBP_Character OtherActor)))
    (Utilities|IsValid _wbp
      (:Is%20Valid
        (Default|HideInteraction _wbp)))))

(event Custom|OnInteraction
  (bind _wbp (Variables|Default|Getwbp))
  (Actor|DestroyActor)
  (Utilities|IsValid _wbp
    (:Is%20Valid
      (Default|HideInteraction _wbp))))

(event EventBeginPlay
  (bind _asbp_hud (Utilities|Casting|CastToBP_HUD (HUD|GetHUD (Game|GetPlayerController 0))))
  (Variables|Default|Setwbp (Variables|/Game/GameManager/BP_HUD.BP_HUD_C|Getwbp _asbp_hud)))

(event Collision|EventActorBeginOverlap
  (params (OtherActor :type Actor%20Object%20Reference)))

(event EventTick
  (params (DeltaSeconds :type Float%20%28single-precision%29)))

(fn ConstructionScript
  (Components|Sphere|SetSphereRadius (Variables|Default|GetSphere) (Variables|Default|GetPickupRadius) true))